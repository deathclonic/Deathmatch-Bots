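; Base game mode that spawns bots and handles respawn after death.
; BeginPlay sorts spawn points into two team lists and a hostile list, then spawns the configured bot count at random navigable points near hostile spawns.
; PlayerDied has the controller possess a temporary spectator at the death spot, then a new bot near a hostile spawn after a delay.
; Team lists go unread here, and DMSpawn and the death-event binding are only in unexecuted nodes.
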(event Custom|PlayerDied
  (params (Character :type Character%20Object%20Reference) (Controller :type Controller%20Object%20Reference))
  (bind _returnvalue (Transformation|GetActorTransform Character))
  (bind _teamspawnshostile (Variables|Default|GetTeamSpawnsHostile))
  (bind _returnvalue_2 (Utilities|Array|LastIndex _teamspawnshostile))
  (bind _returnvalue_3 (Math|Random|RandomIntegerinRange 0 _returnvalue_2))
  (bind _output (Utilities|Array|Get(acopy) _teamspawnshostile _returnvalue_3))
  (bind _returnvalue_4 (Transformation|GetActorTransform _output))
  (Utilities|IsValid Controller
    (:Is%20Valid
      (bind _returnvalue_5 (AI|SpawnAIFromClass "/Game/GAME/BP/BP_SpectatorCharacter.BP_SpectatorCharacter_C" 0 (.location _returnvalue) (.rotation _returnvalue) true 0))
      (Pawn|Possess Controller _returnvalue_5)
      (Utilities|FlowControl|Delay 5.0)
      (bind _randomlocation (Class|NavigationSystemV1|GetRandomLocationinNavigableRadius (.location _returnvalue_4) 2e+02 0 0))
      (bind _returnvalue_6 (AI|SpawnAIFromClass "/Game/GAME/BP/AI/Bot/BP_Bot.BP_Bot_C" 0 _randomlocation (.rotation _returnvalue_4) true 0))
      (Pawn|Possess Controller _returnvalue_6)
      (Actor|DestroyActor _returnvalue_5))))

(event EventBeginPlay
  (bind _teamspawnshostile (Variables|Default|GetTeamSpawnsHostile))
  (bind _botstospawn (Variables|Default|GetBotsToSpawn))
  (bind _returnvalue (Utilities|Array|LastIndex _teamspawnshostile))
  (bind _returnvalue_2 (Math|Random|RandomIntegerinRange 0 _returnvalue))
  (bind _output (Utilities|Array|Get(acopy) _teamspawnshostile _returnvalue_2))
  (bind _returnvalue_3 (Transformation|GetActorTransform _output))
  (bind _outactors (Actor|GetAllActorsOfClass "/Game/GAME/BP/BP_SpawnPoint.BP_SpawnPoint_C"))
  (for _array_element _outactors
    (switch Utilities|FlowControl|Switch|SwitchonE_Teams (Variables|/Game/GAME/BP/BP_SpawnPoint.BP_SpawnPoint_C|GetE_Teams _array_element)
      (:NewEnumerator0
        (Utilities|Array|AddUnique (Variables|Default|GetTeamSpawns1) _array_element))
      (:NewEnumerator1
        (Utilities|Array|AddUnique (Variables|Default|GetTeamSpawns2) _array_element))
      (:NewEnumerator4
        (Utilities|Array|AddUnique (Variables|Default|GetTeamSpawnsHostile) _array_element))))
  (if (> _botstospawn 0)
    (for _index (range 1 _botstospawn)
      (bind _randomlocation (Class|NavigationSystemV1|GetRandomLocationinNavigableRadius (.location _returnvalue_3) 2e+02 0 0))
      (AI|SpawnAIFromClass "/Game/GAME/BP/AI/Bot/BP_Bot.BP_Bot_C" 0 _randomlocation (.rotation _returnvalue_3) true 0))))

(fn ConstructionScript)

(fn DMSpawn
  (params (Controller :type Controller%20Object%20Reference))
  (bind _teamspawnshostile (Variables|Default|GetTeamSpawnsHostile))
  (Utilities|IsValid Controller
    (:Is%20Valid
      (bind _output_get (Variables|Default|SetSelectedSpawn (Utilities|Array|Get(acopy) _teamspawnshostile (Math|Random|RandomIntegerinRange 0 (Utilities|Array|LastIndex _teamspawnshostile)))))
      (bind _randomlocation (Class|NavigationSystemV1|GetRandomLocationinNavigableRadius (.location (Transformation|GetActorTransform _output_get)) 2e+02 0 0))
      (bind _returnvalue (AI|SpawnAIFromClass "/Game/GAME/BP/AI/Bot/BP_Bot.BP_Bot_C" 0 _randomlocation (.rotation (Transformation|GetActorTransform _output_get)) true 0))
      (Pawn|Possess Controller _returnvalue))))