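; AI controller for bots that runs the BT_Bot behavior tree and handles their death and respawn.
; Perception updates set or clear focus and the TargetEnemy and location blackboard keys for sensed BP_BaseCharacter actors.
; Possession starts the brain logic, while unpossession stops it.
; On death it possesses a temporary BP_Spectator, waits a respawn delay, respawns through BP_GameModeBase's DMSpawn, then destroys the spectator.
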(event OnPerceptionUpdated(AIPerception)
  (params (UpdatedActors :type Array%20of%20Actor%20Object%20References))
  (for _array_element UpdatedActors
    _))

(event OnTargetPerceptionUpdated(AIPerception)
  (params (Actor :type Actor%20Object%20Reference) (Stimulus :type AI%20Stimulus%20Structure))
  (bind _bsuccessfullysensed (Utilities|Struct|BreakAIStimulus Stimulus))
  (bind _blackboard (Variables|Default|GetBlackboard))
  (bind _asbp_base_character (Utilities|Casting|CastToBP_BaseCharacter Actor))
  (Utilities|IsValid (Variables|Default|GetBlackboard)
    (:Is%20Valid
      (if _bsuccessfullysensed
        ;[1 1 1] Set focus to the seen character
        (AI|SetFocus _asbp_base_character)
        (AI|Components|Blackboard|SetValueasObject _blackboard (Utilities|Name|MakeLiteralName "TargetEnemy") (select _bsuccessfullysensed _asbp_base_character 0))
        (AI|Components|Blackboard|SetValueasVector _blackboard (Utilities|Name|MakeLiteralName "TargetEnemyLocation") (Transformation|GetWorldLocation (Variables|/Script/Engine.Character|GetMesh _asbp_base_character)))
        (else
          ;[1 1 1] Clear focus
          (AI|ClearFocus)
          (AI|Components|Blackboard|ClearValue (Variables|Default|GetBlackboard) (Utilities|Name|MakeLiteralName "TargetEnemy"))
          (AI|Components|Blackboard|ClearValue (Variables|Default|GetBlackboard) (Utilities|Name|MakeLiteralName "TargetEnemyLocation")))))))

(event Custom|Death
  (params (DeathLocation :type Transform))
  ;[0 1 0] Death
  (bind _returnvalue (AI|SpawnAIFromClass "/Game/GAME/BP/BP_Spectator.BP_Spectator_C" 0 (.location DeathLocation) (.rotation DeathLocation) true 0))
  (Pawn|Possess _returnvalue)
  (CallFunction|StopLogic)
  (Utilities|FlowControl|Delay (Variables|Default|GetRespawnDelay))
  (bind _asbp_game_mode_base (Utilities|Casting|CastToBP_GameModeBase (Game|GetGameMode)))
  (Default|DMSpawn _asbp_game_mode_base self)
  (Utilities|FlowControl|Delay 0.2)
  (Actor|DestroyActor _returnvalue))

(event EventBeginPlay
  ;[1 1 1] Run Behavior
  (Utilities|FlowControl|Delay 0.5)
  (AI|RunBehaviorTree "/Game/GAME/BP/BT_Bot.BT_Bot"))

(event EventPossess
  (params (PossessedPawn :type Pawn%20Object%20Reference))
  (bind _braincomponent (Variables|Default|GetBrainComponent))
  ;[1 1 1] Start logic
  (|CallParentFunction PossessedPawn)
  (Utilities|IsValid _braincomponent
    (:Is%20Valid
      (AI|Logic|StartLogic _braincomponent))))

(event EventUnPossess
  (params (UnpossessedPawn :type Pawn%20Object%20Reference))
  ;[1 1 1] Stop logic
  (|CallParentFunction UnpossessedPawn)
  (CallFunction|StopLogic))

(fn ConstructionScript)

(fn StopLogic
  (bind _returnvalue (AI|GetBlackboard 0))
  (Utilities|IsValid _returnvalue
    (:Is%20Valid
      (AI|Components|Blackboard|ClearValue _returnvalue (Utilities|Name|MakeLiteralName "TargetEnemy"))
      (AI|Logic|StopLogic (Variables|Default|GetBrainComponent) "Dead"))))