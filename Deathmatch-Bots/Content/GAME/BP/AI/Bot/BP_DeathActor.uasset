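; BP_DeathActor is a physics death prop in the AI Bot folder that displays a given static mesh and launches it along a character's last motion.
; On BeginPlay it sets the mesh and, if the CharacterMovement reference is valid, applies a velocity-change impulse of the last update velocity plus RagdollImpulseStrength in that direction.
; The SetSimulatePhysics call is unconnected, so the graph itself never enables physics.
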(event EventBeginPlay
  (Components|StaticMesh|SetStaticMesh (Variables|Default|GetStaticMesh) (Variables|Default|GetNew%20Mesh))
  (bind _charactermovement (Variables|Default|GetCharacterMovement)
    (:then
      (Physics|AddImpulse (Variables|Default|GetStaticMesh) (+ (Pawn|Components|CharacterMovement|GetLastUpdateVelocity _charactermovement) (* (Math|Vector|Normalize (Pawn|Components|CharacterMovement|GetLastUpdateVelocity _charactermovement)) (Variables|Default|GetRagdollImpulseStrength))) "None" true))
    (:else)))

(event Collision|EventActorBeginOverlap
  (params (OtherActor :type Actor%20Object%20Reference)))

(event EventTick
  (params (DeltaSeconds :type Float%20%28single-precision%29)))

(fn ConstructionScript)