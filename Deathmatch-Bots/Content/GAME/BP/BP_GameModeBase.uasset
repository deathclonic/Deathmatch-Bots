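; Game mode that handles bot spawning and deathmatch-style spawns.
; Shortly after BeginPlay it caches BP_SpawnPoint actors into Hostile, Team 1 and Team 2 lists, then spawns BotsToSpawn BP_Bots.
; DMSpawn creates a BP_Bot and has the supplied controller possess it.
; Both spawn paths use only Hostile points, choosing a random nearby navigable location raised off the floor.
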(event EventTick
  (params (DeltaSeconds :type Float%20%28single-precision%29)))

(event EventBeginPlay
  (bind _teamspawnshostile (Variables|Default|GetTeamSpawnsHostile))
  (bind _botstospawn (Variables|Default|GetBotsToSpawn))
  (bind _returnvalue (Utilities|Array|LastIndex _teamspawnshostile))
  (bind _returnvalue_2 (Math|Random|RandomIntegerinRange 0 _returnvalue))
  (bind _output (Utilities|Array|Get(acopy) _teamspawnshostile _returnvalue_2))
  (bind _returnvalue_3 (Transformation|GetActorTransform _output))
  ;[0 1 0] Begin Play
  (Utilities|FlowControl|Delay 0.2)
  ;[1 1 1] Cache the spawn points and set teams
  (bind _outactors (Actor|GetAllActorsOfClass "/Game/GAME/BP/BP_SpawnPoint.BP_SpawnPoint_C"))
  (for _array_element _outactors
    (switch Utilities|FlowControl|Switch|SwitchonE_Teams (Variables|/Game/GAME/BP/BP_SpawnPoint.BP_SpawnPoint_C|GetE_Teams _array_element)
      (:NewEnumerator1
        (Utilities|Array|AddUnique (Variables|Default|GetTeamSpawnsHostile) _array_element))
      (:NewEnumerator2
        (Utilities|Array|AddUnique (Variables|Default|GetTeamSpawns1) _array_element))
      (:NewEnumerator3
        (Utilities|Array|AddUnique (Variables|Default|GetTeamSpawns2) _array_element))))
  ;[1 1 1] Initial spawning
  (if (> _botstospawn 0)
    (for _index (range 1 _botstospawn)
      (bind _randomlocation (Class|NavigationSystemV1|GetRandomLocationinNavigableRadius (.location _returnvalue_3) 2e+02 0 0))
      (bind _returnvalue_4 (AI|SpawnAIFromClass "/Game/GAME/BP/BP_Bot.BP_Bot_C" 0 (+ _randomlocation "0.000000,0.000000,50.000000") (.rotation _returnvalue_3) true 0)))))

(fn ConstructionScript)

(fn DMSpawn
  (params (Controller :type Controller%20Object%20Reference))
  (bind _teamspawnshostile (Variables|Default|GetTeamSpawnsHostile))
  (bind _returnvalue (Utilities|Array|LastIndex _teamspawnshostile))
  (bind _returnvalue_2 (Math|Random|RandomIntegerinRange 0 _returnvalue))
  (bind _output (Utilities|Array|Get(acopy) _teamspawnshostile _returnvalue_2))
  (bind _returnvalue_3 (Transformation|GetActorTransform _output))
  (Utilities|IsValid Controller
    (:Is%20Valid
      (bind _randomlocation (Class|NavigationSystemV1|GetRandomLocationinNavigableRadius (.location _returnvalue_3) 2e+02 0 0))
      (bind _returnvalue_4 (AI|SpawnAIFromClass "/Game/GAME/BP/BP_Bot.BP_Bot_C" 0 (+ _randomlocation "0.000000,0.000000,100.000000") (.rotation _returnvalue_3) true 0))
      (Pawn|Possess Controller _returnvalue_4))))