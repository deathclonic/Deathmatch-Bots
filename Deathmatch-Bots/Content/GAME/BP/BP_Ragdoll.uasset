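; BP_Ragdoll is a Blueprint that switches a skeletal mesh into ragdoll physics through its ActivateRagdoll event.
; The event applies the Ragdoll collision profile and simulates physics on the impulse bone and all bodies below it.
; It then launches that bone with a velocity-change impulse built from the character movement's last velocity plus extra strength along that direction.
; A delayed step to stop simulation is disconnected and never runs.
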(event Custom|ActivateRagdoll
  (params (CharacterMovement :type Character%20Movement%20Component%20Object%20Reference))
  (bind _returnvalue (Pawn|Components|CharacterMovement|GetLastUpdateVelocity CharacterMovement))
  (bind _ragdollimpulsebone (Variables|Default|GetRagdollImpulseBone))
  (bind _skeletalmesh (Variables|Default|GetSkeletalMesh))
  ;[1 1 1] Activate Character Physics
  (Collision|SetCollisionProfileName _skeletalmesh "Ragdoll" true :!class /Script/Engine.PrimitiveComponent)
  (Class|SkeletalMeshComponent|SetAllBodiesBelowSimulatePhysics _skeletalmesh _ragdollimpulsebone true true)
  (Physics|AddImpulse _skeletalmesh (+ _returnvalue (* (Math|Vector|Normalize _returnvalue) (Variables|Default|GetRagdollImpulseStrength))) _ragdollimpulsebone true))

(fn ConstructionScript)